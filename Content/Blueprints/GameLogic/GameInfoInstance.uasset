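; Game Instance for a jigsaw puzzle game, holding session choices, points, store and purchased puzzles, user preferences, and persistent music.
; Each data set saves to its own slot through a shared GameSave_BP object; Init loads points, store, purchases and preferences.
; In-progress and completed puzzles fill the first (Continue) and last (Gallery) category entries.
; Saving progress overwrites matching image and piece-count entries, else appends and passes the new index to the puzzle widget.
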(event EventSetChosenPuzzleImage
  (params (Chosen%20Image :type Texture%202D%20Object%20Reference))
  ;[1 1 1] Set Chosen Image
  (Variables|Texture2D|SetChosen%20Puzzle%20Image Chosen%20Image))

(event EventSetNumberOfPieces
  (params (Number%20Of%20Pieces :type Integer))
  ;[1 1 1] Set Number Of Pieces
  (Variables|Integers|SetNumber%20Of%20Pieces Number%20Of%20Pieces))

(event EventSetBaseMixSFX
  (bind _user_preferences (Variables|Structs|GetUser%20Preferences))
  (bind (_sfxmuted _sfxvolume) (Utilities|Struct|BreakUserPreferences _user_preferences))
  (bind _returnvalue (select _sfxmuted "/Game/Sounds/Mixes/MuteSFX.MuteSFX" "/Game/Sounds/Mixes/UnmuteSFX.UnmuteSFX"))
  ;[1 1 1] Set Base Mix for SFX Based On User Prefrences
  (Audio|SetSoundMixClassOverride _returnvalue "/Game/Sounds/Classes/SFX_SC.SFX_SC" (select _sfxmuted 0.0 _sfxvolume) 1.0 1.0 true)
  (Class|GameplayStatics|SetBaseSoundMix _returnvalue))

(event EventSetUserPreferences
  (params (User%20Preferences :type User%20Preferences%20Structure))
  ;[1 1 1] Set User Prefrences
  (Variables|Structs|SetUser%20Preferences User%20Preferences))

(event EventSetStorePuzzles
  (params (Store%20Puzzles :type Array%20of%20Store%20Puzzles%20Structures))
  ;[1 1 1] Override Store Puzzles and Purchased Puzzles Array
  (Variables|Structs|SetStore%20Puzzles Store%20Puzzles))

(event EventSetPurchasedPuzzles
  (params (New%20Category%20Data :type Array%20of%20Category%20Data%20Struct%20Structures))
  ;[1 1 1] Override Store Puzzles and Purchased Puzzles Array
  (Variables|Structs|SetCategories%20Data%20Struct New%20Category%20Data))

(event EventSetGameTime
  (params (Game%20Time :type Integer))
  ;[1 1 1] Set Game Time
  (Variables|Integers|SetGame%20Time Game%20Time))

(event EventSetPuzzleCategory
  (params (Puzzle%20Category :type Categories%20Enum :default "NewEnumerator7"))
  ;[1 1 1] Set Puzzle Category
  (Variables|Enums|SetCategory Puzzle%20Category))

(event EventPopulateContinueCategory
  (bind _categories_data_struct (Variables|Structs|GetCategories%20Data%20Struct))
  (bind _output (Utilities|Array|Get(acopy) _categories_data_struct))
  (bind _textures (Utilities|Struct|BreakCategoryDataStruct _output))
  ;[1 1 1] Populate Continue Category
  (Utilities|FlowControl|Sequence
    (:then_0
      (Utilities|Array|Clear (Utilities|Struct|BreakCategoryDataStruct (Utilities|Array|Get(acopy) (Variables|Structs|GetCategories%20Data%20Struct)))))
    (:then_1
      (bind _loaded (CallFunction|LoadCurrentPuzzleProgression))
      (if _loaded
        (for _array_element (Variables|Structs|GetPuzzles%20In%20Progress)
          (if (not (Utilities|Array|ContainsItem _textures (Utilities|Struct|BreakPuzzlesInProgressStruct _array_element)))
            (Utilities|Array|Add _textures (Utilities|Struct|BreakPuzzlesInProgressStruct _array_element))))))))

(event EventPopulateGalleryCategory
  (bind _categories_data_struct (Variables|Structs|GetCategories%20Data%20Struct))
  (bind _returnvalue (Utilities|Array|LastIndex _categories_data_struct))
  (bind _output (Utilities|Array|Get(acopy) _categories_data_struct _returnvalue))
  (bind _textures (Utilities|Struct|BreakCategoryDataStruct _output))
  ;[1 1 1] Populate Gallery Category from Category Data Struct with Completed Puzzles -- Called in Main Menu Game Mode on BeginPlay
  (bind _loaded (CallFunction|LoadCompletedPuzzles))
  (if _loaded
    (Utilities|FlowControl|Sequence
      (:then_0
        (Utilities|Array|Clear _textures))
      (:then_1
        (for _array_element (Variables|Structs|GetCompleted%20Puzzles)
          (Utilities|Array|Add _textures (Utilities|Struct|BreakPuzzlesCompletedStruct _array_element)))))))

(event EventSetReward
  (params (Reward :type Integer))
  (Variables|Integers|SetReward Reward))

(event EventSetTotalPoints
  (params (Reward%20Points :type Integer))
  ;[1 1 1] Set Total Points
  (Variables|Integers|SetTotal%20Points (+ Reward%20Points (Variables|Integers|GetTotal%20Points))))

(event EventSpawnMusic
  (params (Volume :type Float%20%28double-precision%29))
  ;[1 1 1] Spawn Music
  (Utilities|IsValid (Variables|Default|GetMusic%20Component)
    (:Is%20Not%20Valid
      (bind _returnvalue (Audio|SpawnSound2D "/Game/Sounds/Cues/Komiku_-_12_-_Bicycle_Cue.Komiku_-_12_-_Bicycle_Cue" 1.0 1.0 0.0 0 true false))
      (bind _output_get (Variables|Default|SetMusic%20Component _returnvalue))
      (Audio|Components|Audio|SetVolumeMultiplier _output_get Volume :!class /Script/Engine.AudioComponent))))

(event EventInit
  ;[1 1 1] Event Init
  (CallFunction|LoadTotalPoints)
  (CallFunction|LoadStorePuzzles)
  (CallFunction|LoadPurchasedPuzzles)
  (bind _loaded (CallFunction|LoadUserPreferences))
  (if _loaded
    (CallFunction|SetGameTime (Utilities|Struct|BreakUserPreferences (Variables|Structs|GetUser%20Preferences)))))

(fn DeleteCurrentPuzzleProgression
  (params (Puzzle%20Index :type Integer))
  (bind _puzzles_in_progress (Variables|Structs|GetPuzzles%20In%20Progress))
  (Utilities|FlowControl|Sequence
    (:then_0
      (if (Utilities|Array|IsValidIndex _puzzles_in_progress Puzzle%20Index)
        (Utilities|Array|RemoveItem _puzzles_in_progress (Utilities|Array|Get(acopy) _puzzles_in_progress Puzzle%20Index))
        (Utilities|IsValid (Variables|Refs|GetSave%20Game%20Ref)
          (:Is%20Valid
            _)
          (:Is%20Not%20Valid
            (bind _returnvalue (SaveGame|CreateSaveGameObject "/Game/Blueprints/GameLogic/GameSave_BP.GameSave_BP_C"))
            (Variables|Refs|SetSave%20Game%20Ref _returnvalue)))
        (bind _output_get (Variables|/Game/Blueprints/GameLogic/GameSave_BP.GameSave_BP_C|SetPuzzle%20In%20Progress (Variables|Refs|GetSave%20Game%20Ref) (Variables|Structs|GetPuzzles%20In%20Progress)))
        (if (== (Utilities|Array|Length _output_get) 0)
          (bind _returnvalue_2 (SaveGame|DeleteGameinSlot "PuzzlesInProgress"))
          (LocalVariables|SetDeleted%20-%20LV _returnvalue_2)
          (else
            (bind _returnvalue_3 (SaveGame|SaveGametoSlot (Variables|Refs|GetSave%20Game%20Ref) "PuzzlesInProgress"))
            (LocalVariables|SetDeleted%20-%20LV _returnvalue_3)))))
    (:then_1
      (CallFunction|PopulateContinueCategory)
      (return (LocalVariables|GetDeleted%20-%20LV)))))

(fn LoadCompletedPuzzles
  (bind _returnvalue (SaveGame|DoesSaveGameExist "CompletedPuzzles"))
  (if _returnvalue
    (bind _returnvalue_2 (SaveGame|LoadGamefromSlot "CompletedPuzzles"))
    (bind _game_save_ref (Class|GameSaveInterface|ReturnSelf(Message) _returnvalue_2))
    (Variables|Structs|SetCompleted%20Puzzles (Variables|/Game/Blueprints/GameLogic/GameSave_BP.GameSave_BP_C|GetCompleted%20Puzzles _game_save_ref))
    (return true)
    (else
      (return false))))

(fn LoadCurrentPuzzleProgression
  (bind _returnvalue (SaveGame|DoesSaveGameExist "PuzzlesInProgress"))
  (if _returnvalue
    (bind _returnvalue_2 (SaveGame|LoadGamefromSlot "PuzzlesInProgress"))
    (bind _game_save_ref (Class|GameSaveInterface|ReturnSelf(Message) _returnvalue_2))
    (Variables|Structs|SetPuzzles%20In%20Progress (Variables|/Game/Blueprints/GameLogic/GameSave_BP.GameSave_BP_C|GetPuzzle%20In%20Progress _game_save_ref))
    (return true)
    (else
      (return false))))

(fn LoadPurchasedPuzzles
  (bind _returnvalue (SaveGame|DoesSaveGameExist "PurchasedPuzzles"))
  (if _returnvalue
    (bind _returnvalue_2 (SaveGame|LoadGamefromSlot "PurchasedPuzzles"))
    (bind _game_save_ref (Class|GameSaveInterface|ReturnSelf(Message) _returnvalue_2))
    (Variables|Structs|SetCategories%20Data%20Struct (Variables|/Game/Blueprints/GameLogic/GameSave_BP.GameSave_BP_C|GetPuzzles _game_save_ref))
    (return true)
    (else
      (return false))))

(fn LoadStorePuzzles
  (bind _returnvalue (SaveGame|DoesSaveGameExist "StorePuzzles"))
  (if _returnvalue
    (bind _returnvalue_2 (SaveGame|LoadGamefromSlot "StorePuzzles"))
    (bind _game_save_ref (Class|GameSaveInterface|ReturnSelf(Message) _returnvalue_2))
    (Variables|Structs|SetStore%20Puzzles (Variables|/Game/Blueprints/GameLogic/GameSave_BP.GameSave_BP_C|GetStore%20Puzzles _game_save_ref))
    (return true)
    (else
      (return false))))

(fn LoadTotalPoints
  (bind _returnvalue (SaveGame|DoesSaveGameExist "TotalPoints"))
  (if _returnvalue
    (bind _returnvalue_2 (SaveGame|LoadGamefromSlot "TotalPoints"))
    (bind _game_save_ref (Class|GameSaveInterface|ReturnSelf(Message) _returnvalue_2))
    (Variables|Integers|SetTotal%20Points (Variables|/Game/Blueprints/GameLogic/GameSave_BP.GameSave_BP_C|GetTotal%20Points _game_save_ref))
    (return true)
    (else
      (return false))))

(fn LoadUserPreferences
  (bind _returnvalue (SaveGame|DoesSaveGameExist "UserPreferences"))
  (if _returnvalue
    (bind _returnvalue_2 (SaveGame|LoadGamefromSlot "UserPreferences"))
    (bind _game_save_ref (Class|GameSaveInterface|ReturnSelf(Message) _returnvalue_2))
    (Variables|Structs|SetUser%20Preferences (Variables|/Game/Blueprints/GameLogic/GameSave_BP.GameSave_BP_C|GetUser%20Preferences _game_save_ref))
    (return true)
    (else
      (return false))))

(fn ReturnBackgroundColors
  (return (Variables|LinearColors|GetBackground%20Colors)))

(fn ReturnCategoryStructArray
  (return (Variables|Structs|GetCategories%20Data%20Struct)))

(fn ReturnChosenPuzzleImage
  (return (Variables|Texture2D|GetChosen%20Puzzle%20Image)))

(fn ReturnCompletedPuzzles
  (return (Variables|Structs|GetCompleted%20Puzzles)))

(fn ReturnCurrentPuzzleProgression
  (return (Variables|Structs|GetPuzzles%20In%20Progress)))

(fn ReturnGameTime
  (return (Variables|Integers|GetGame%20Time)))

(fn ReturnMusicComponent
  (return (Variables|Default|GetMusic%20Component)))

(fn ReturnNumberOfPieces
  (return (Variables|Integers|GetNumber%20Of%20Pieces)))

(fn ReturnPuzzleCategory
  (return (Variables|Enums|GetCategory)))

(fn ReturnReward
  (return (Variables|Integers|GetReward)))

(fn ReturnSelectedBackgroundColor
  (return (Utilities|Struct|BreakUserPreferences (Variables|Structs|GetUser%20Preferences))))

(fn ReturnStorePuzzles
  (return (Variables|Structs|GetStore%20Puzzles)))

(fn ReturnTotalPoints
  (return (Variables|Integers|GetTotal%20Points)))

(fn ReturnUserPreferences
  (return (Variables|Structs|GetUser%20Preferences)))

(fn SaveCompletedPuzzles
  (params (Completed%20Puzzle%20Struct :type Puzzles%20Completed%20Struct%20Structure))
  (Utilities|IsValid (Variables|Refs|GetSave%20Game%20Ref)
    (:Is%20Valid
      _)
    (:Is%20Not%20Valid
      (bind _returnvalue (SaveGame|CreateSaveGameObject "/Game/Blueprints/GameLogic/GameSave_BP.GameSave_BP_C"))
      (Variables|Refs|SetSave%20Game%20Ref _returnvalue)))
  (bind _array_element (Utilities|Array|ForEachLoopwithBreak (Variables|Structs|GetCompleted%20Puzzles) :!label _label)
    (:LoopBody
      (if (Utilities|Enum|Equal(Enum) (Utilities|GetDisplayName (Utilities|Struct|BreakPuzzlesCompletedStruct _array_element)) (Utilities|GetDisplayName (Utilities|Struct|BreakPuzzlesCompletedStruct Completed%20Puzzle%20Struct)))
        (Utilities|FlowControl|Sequence
          (:then_0
            (goto _label Break))
          (:then_1
            (LocalVariables|SetFound true)))))
    (:Completed
      (if (not (LocalVariables|GetFound))
        (Utilities|Array|Add (Variables|Structs|GetCompleted%20Puzzles) Completed%20Puzzle%20Struct)
        (Variables|/Game/Blueprints/GameLogic/GameSave_BP.GameSave_BP_C|SetCompleted%20Puzzles (Variables|Refs|GetSave%20Game%20Ref) (Variables|Structs|GetCompleted%20Puzzles))
        (bind _returnvalue_2 (SaveGame|SaveGametoSlot (Variables|Refs|GetSave%20Game%20Ref) "CompletedPuzzles"))
        (return _returnvalue_2)))))

(fn SaveCurrentPuzzleProgression
  (params (Current%20Puzzle%20 :type Puzzles%20in%20Progress%20Struct%20Structure) (Puzzle%20Index :type Integer))
  (bind (_puzzleimage _numberofpieces) (Utilities|Struct|BreakPuzzlesInProgressStruct Current%20Puzzle%20))
  (LocalVariables|SetPuzzle%20Index%20-%20LV Puzzle%20Index)
  (Utilities|IsValid (Variables|Refs|GetSave%20Game%20Ref)
    (:Is%20Valid
      _)
    (:Is%20Not%20Valid
      (bind _returnvalue (SaveGame|CreateSaveGameObject "/Game/Blueprints/GameLogic/GameSave_BP.GameSave_BP_C"))
      (Variables|Refs|SetSave%20Game%20Ref _returnvalue)))
  (if (!= (LocalVariables|GetPuzzle%20Index%20-%20LV) -1)
    (Utilities|Array|SetArrayElem (Variables|Structs|GetPuzzles%20In%20Progress) (LocalVariables|GetPuzzle%20Index%20-%20LV) Current%20Puzzle%20 :!label _label)
    (Variables|/Game/Blueprints/GameLogic/GameSave_BP.GameSave_BP_C|SetPuzzle%20In%20Progress (Variables|Refs|GetSave%20Game%20Ref) (Variables|Structs|GetPuzzles%20In%20Progress) :!label _label_2)
    (bind _returnvalue_2 (SaveGame|SaveGametoSlot (Variables|Refs|GetSave%20Game%20Ref) "PuzzlesInProgress"))
    (return _returnvalue_2)
    (else
      (bind (_array_element _array_index) (Utilities|Array|ForEachLoopwithBreak (Variables|Structs|GetPuzzles%20In%20Progress) :!label _label_3)
        (:LoopBody
          (if (and (== (.PuzzleImage (Utilities|Struct|BreakPuzzlesInProgressStruct _array_element)) _puzzleimage) (== (.NumberOfPieces (Utilities|Struct|BreakPuzzlesInProgressStruct _array_element)) _numberofpieces))
            (Utilities|FlowControl|Sequence
              (:then_0
                (goto _label_3 Break))
              (:then_1
                (LocalVariables|SetPuzzle%20Index%20-%20LV _array_index)
                (LocalVariables|SetFound true)
                (goto _label)))))
        (:Completed
          (if (not (LocalVariables|GetFound))
            (bind _returnvalue_3 (Utilities|Array|Add (Variables|Structs|GetPuzzles%20In%20Progress) Current%20Puzzle%20))
            (bind _puzzle_wb (Class|GamePlayGMInterface|ReturnPuzzleWB(Message) (Game|GetGameMode)))
            (Variables|/Game/Blueprints/UI/GamePlay/Puzzle_WB.Puzzle_WB_C|SetPuzzle%20Index _puzzle_wb _returnvalue_3)
            (goto _label_2)))))))

(fn SavePurchasedPuzzles
  (Utilities|IsValid (Variables|Refs|GetSave%20Game%20Ref)
    (:Is%20Valid
      _)
    (:Is%20Not%20Valid
      (bind _returnvalue (SaveGame|CreateSaveGameObject "/Game/Blueprints/GameLogic/GameSave_BP.GameSave_BP_C"))
      (Variables|Refs|SetSave%20Game%20Ref _returnvalue)))
  (Variables|/Game/Blueprints/GameLogic/GameSave_BP.GameSave_BP_C|SetPuzzles (Variables|Refs|GetSave%20Game%20Ref) (Variables|Structs|GetCategories%20Data%20Struct))
  (bind _returnvalue_2 (SaveGame|SaveGametoSlot (Variables|Refs|GetSave%20Game%20Ref) "PurchasedPuzzles"))
  (return _returnvalue_2))

(fn SaveStorePuzzles
  (Utilities|IsValid (Variables|Refs|GetSave%20Game%20Ref)
    (:Is%20Valid
      _)
    (:Is%20Not%20Valid
      (bind _returnvalue (SaveGame|CreateSaveGameObject "/Game/Blueprints/GameLogic/GameSave_BP.GameSave_BP_C"))
      (Variables|Refs|SetSave%20Game%20Ref _returnvalue)))
  (Variables|/Game/Blueprints/GameLogic/GameSave_BP.GameSave_BP_C|SetStore%20Puzzles (Variables|Refs|GetSave%20Game%20Ref) (Variables|Structs|GetStore%20Puzzles))
  (bind _returnvalue_2 (SaveGame|SaveGametoSlot (Variables|Refs|GetSave%20Game%20Ref) "StorePuzzles"))
  (return _returnvalue_2))

(fn SaveTotalPoints
  (Utilities|IsValid (Variables|Refs|GetSave%20Game%20Ref)
    (:Is%20Valid
      _)
    (:Is%20Not%20Valid
      (bind _returnvalue (SaveGame|CreateSaveGameObject "/Game/Blueprints/GameLogic/GameSave_BP.GameSave_BP_C"))
      (Variables|Refs|SetSave%20Game%20Ref _returnvalue)))
  (Variables|/Game/Blueprints/GameLogic/GameSave_BP.GameSave_BP_C|SetTotal%20Points (Variables|Refs|GetSave%20Game%20Ref) (Variables|Integers|GetTotal%20Points))
  (bind _returnvalue_2 (SaveGame|SaveGametoSlot (Variables|Refs|GetSave%20Game%20Ref) "TotalPoints"))
  (return _returnvalue_2))

(fn SaveUserPreferences
  (Utilities|IsValid (Variables|Refs|GetSave%20Game%20Ref)
    (:Is%20Valid
      _)
    (:Is%20Not%20Valid
      (bind _returnvalue (SaveGame|CreateSaveGameObject "/Game/Blueprints/GameLogic/GameSave_BP.GameSave_BP_C"))
      (bind _output_get (Variables|Refs|SetSave%20Game%20Ref _returnvalue))))
  (Variables|/Game/Blueprints/GameLogic/GameSave_BP.GameSave_BP_C|SetUser%20Preferences _output_get (Variables|Structs|GetUser%20Preferences))
  (bind _returnvalue_2 (SaveGame|SaveGametoSlot (Variables|Refs|GetSave%20Game%20Ref) "UserPreferences"))
  (return _returnvalue_2))