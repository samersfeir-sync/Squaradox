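; Main menu game mode that sets up the front end when the level begins play.
; BeginPlay asks the game instance to populate the Continue and Gallery categories, then creates the main menu widget and adds it to the viewport.
; It reads user preferences from the game instance to start music at the saved or muted volume and applies the base SFX mix, all through game instance message calls.
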(event EventBeginPlay
  (bind _returnvalue (Game|GetGameInstance))
  (Utilities|FlowControl|Sequence
    (:then_0
      (Class|GameInstanceInterface|PopulateContinueCategory(Message) (Game|GetGameInstance)))
    (:then_1
      (Class|GameInstanceInterface|PopulateGalleryCategory(Message) (Game|GetGameInstance)))
    (:then_2
      (bind _returnvalue_2 (UserInterface|CreateWidget "/Game/Blueprints/UI/MainMenu/MainMenu_WB.MainMenu_WB_C"))
      (UserInterface|Viewport|AddtoViewport _returnvalue_2 0)
      (bind _user_preferences (Class|GameInstanceInterface|ReturnUserPreferences(Message) _returnvalue))
      (Class|GameInstanceInterface|SpawnMusic(Message) _returnvalue (select (.MusicMuted (Utilities|Struct|BreakUserPreferences _user_preferences)) 0.0 (.MusicVolume (Utilities|Struct|BreakUserPreferences _user_preferences))))
      (Class|GameInstanceInterface|SetBaseMixSFX(Message) _returnvalue))))

(fn ConstructionScript)